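; DebugEnemy is an enemy Blueprint, apparently for debugging, that displays its health on a material billboard bar.
; The construction script creates a dynamic instance of MI_HealthBar at full health and assigns it to the bar.
; Each Tick feeds the current-to-full health ratio into the material's Health parameter and rebuilds the sprite element to scale its height.
; A ResettoDefaultValues event restores health and movement speed.
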(event EventBeginPlay)

(event Collision|EventActorBeginOverlap
  (params (OtherActor :type Actor%20Object%20Reference)))

(event EventTick
  (params (DeltaSeconds :type Float%20%28single-precision%29))
  (bind _currenthealth (Variables|Default|GetCurrentHealth))
  (bind _fullhealth (Variables|Default|Getfullhealth))
  (bind _healthbar (Variables|Default|GetHealthBar))
  (bind _returnvalue (/ _currenthealth _fullhealth))
  (bind _elements (Variables|/Script/Engine.MaterialBillboardComponent|GetElements _healthbar))
  (bind _output (Utilities|Array|Get(acopy) _elements))
  (bind (_material _distancetoopacitycurve _bsizeisinscreenspace _basesizex _basesizey _distancetosizecurve) (Utilities|Struct|BreakMaterialSpriteElement _output))
  (Rendering|Material|SetScalarParameterValue (Variables|Default|Getmaterial) "Health" _returnvalue :!class /Script/Engine.MaterialInstanceDynamic)
  (Utilities|Array|SetArrayElem _elements 0 (Utilities|Struct|MakeMaterialSpriteElement _material _distancetoopacitycurve _bsizeisinscreenspace _basesizex (* _returnvalue 32.0) _distancetosizecurve)))

(event EventResettoDefaultValues
  (bind _output_get (Variables|Default|SetCurrentHealth 1e+01))
  (Variables|Default|Setfullhealth _output_get)
  (Variables|Default|SetMovementSpeed 0.1))

(fn ConstructionScript
  (bind _returnvalue (Rendering|Material|CreateDynamicMaterialInstance "/Game/Material/HealthBar/MI_HealthBar.MI_HealthBar" "None" "None" :!class /Script/Engine.KismetMaterialLibrary))
  (bind _output_get (Variables|Default|Setmaterial _returnvalue))
  (Rendering|Material|SetScalarParameterValue _returnvalue "Health" 1.0 :!class /Script/Engine.MaterialInstanceDynamic)
  (Rendering|Material|SetMaterial (Variables|Default|GetHealthBar) 0 _output_get))