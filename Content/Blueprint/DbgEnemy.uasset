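; DbgEnemy is an enemy Blueprint, apparently for debugging, that displays its health on a material billboard bar.
; The construction script creates a dynamic instance of MI_HealthBar, starts it at full health and assigns it to HealthBar.
; Every Tick writes CurrentHealth, scaled against a hardcoded maximum, to the material's Health parameter and rebuilds the billboard's sprite element.
; The graph only displays CurrentHealth and never changes it.
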(event EventBeginPlay)

(event Collision|EventActorBeginOverlap
  (params (OtherActor :type Actor%20Object%20Reference)))

(event EventTick
  (params (DeltaSeconds :type Float%20%28single-precision%29))
  (Rendering|Material|SetScalarParameterValue (Variables|Default|GetMat) "Health" (/ (Variables|Default|GetCurrentHealth) 1e+01) :!class /Script/Engine.MaterialInstanceDynamic)
  (Class|MaterialBillboardComponent|SetElements (Variables|Default|GetHealthBar) (Utilities|Array|MakeArray (Utilities|Struct|MakeMaterialSpriteElement (Variables|Default|GetMat) 0 false 32.0 6.0))))

(fn ConstructionScript
  (bind _returnvalue (Rendering|Material|CreateDynamicMaterialInstance "/Game/Material/HealthBar/MI_HealthBar.MI_HealthBar" "None" "None" :!class /Script/Engine.KismetMaterialLibrary))
  (bind _output_get (Variables|Default|SetMat _returnvalue))
  (Rendering|Material|SetScalarParameterValue _output_get "Health" 1.0 :!class /Script/Engine.MaterialInstanceDynamic)
  (Rendering|Material|SetMaterial (Variables|Default|GetHealthBar) 0 _output_get))